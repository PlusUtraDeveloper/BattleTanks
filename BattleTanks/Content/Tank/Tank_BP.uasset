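; Player-controllable tank Blueprint that wires its components together and routes input to them.
; On BeginPlay it hands the barrel and turret to the Aiming component and both tracks to TankMovement.
; Move and turn axes pass intent to TankMovement, and the Fire action calls Aiming.
; Aim axes orbit the view with frame-time-scaled rotation, splitting yaw onto an azimuth gimbal and pitch onto the spring arm.
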(event `self.ReceiveBeginPlay`
  (`AimingComponent.Initialise` (`self.Aiming`) (`self.Barrel`) (`self.Turrent`))
  (`TankMovementComponent.Initialise` (`self.TankMovement`) (`self.LeftTrack`) (`self.RightTrack`)))

(event `InputAxis|AimAzimuth`
  (params (AxisValue :type "Float (single-precision)"))
  ;[1 1 1] Aim Input Setup
  (`SceneComponent.K2_AddLocalRotation` (`self.Azimuth Gimbal`) (`KismetMathLibrary.MakeRotator` 0.0 0.0 (* AxisValue (`GameplayStatics.GetWorldDeltaSeconds`) 100.0)) false false))

(event `InputAxis|Move Forward`
  (params (AxisValue :type "Float (single-precision)"))
  ;[1 1 1] Movement Input Setup
  (`TankMovementComponent.IntendMoveForward` (`self.TankMovement`) AxisValue))

(event `InputAxis|Turn Right`
  (params (AxisValue :type "Float (single-precision)"))
  ;[1 1 1] Movement Input Setup
  (`TankMovementComponent.IntendTurnRight` (`self.TankMovement`) AxisValue))

(event `InputAxis|AimAltitude`
  (params (AxisValue :type "Float (single-precision)"))
  ;[1 1 1] Aim Input Setup
  (`SceneComponent.K2_AddLocalRotation` (`self.SpringArm`) (`KismetMathLibrary.MakeRotator` 0.0 (* AxisValue (`GameplayStatics.GetWorldDeltaSeconds`) 100.0)) false false))

(event `InputAction|Fire`
  (params (Key :type "Key Structure" :default "AnyKey"))
  ;[1 1 1] Aim Input Setup
  (:`Pressed`
    (`AimingComponent.Fire` (`self.Aiming`))))

(fn `UserConstructionScript`)